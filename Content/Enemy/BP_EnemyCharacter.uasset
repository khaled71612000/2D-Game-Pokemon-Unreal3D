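; Enemy character that is squashed when the player collides with it, bouncing the player upward.
; A capsule hit from BP_Player launches the player up and calls Squash.
; The OnSquashed event spawns an explosion effect, destroys the actor and plays a squash sound.
; The hit condition is hardwired true, so any player contact counts; the velocity-based IsSquashHit check is left unconnected.
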(event `self.CapsuleComponent.OnComponentHit`
  (params (HitComponent :type "PrimitiveComponent Object Reference") (OtherActor :type "Actor Object Reference") (OtherComp :type "PrimitiveComponent Object Reference") (NormalImpulse :type "Vector Structure") (Hit :type "HitResult Structure (by ref)"))
  (if true
    (bind _asbp_player (cast `/Game/Character/BP_Player` OtherActor))
    (`self.LaunchCharacter` _asbp_player (0.0 0.0 400.0) false false)
    (`self.Squash` 1.0)))

(event `self.OnSquashed`
  (bind _returnvalue (`self.K2_GetActorLocation`))
  (`NiagaraFunctionLibrary.SpawnSystemAtLocation` "/Niagara/DefaultAssets/Templates/Systems/SimpleExplosion.SimpleExplosion" _returnvalue)
  (`self.K2_DestroyActor`)
  (`GameplayStatics.PlaySoundAtLocation` "/Game/Character/Squash.Squash" _returnvalue (struct) 1.0 1.0 0.0 null null null null))

(fn `UserConstructionScript`)